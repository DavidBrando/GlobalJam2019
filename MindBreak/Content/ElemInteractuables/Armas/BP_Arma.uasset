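; BP_Arma is a base weapon among the game's interactable items, with empty Disparar (fire) and Recargar (reload) events that child weapons can override.
; Its construction script runs the parent's, flags the weapon as pickable and sets the weapon type to the enum's first entry.
; It also writes the InfoDelArma struct, covering damage, ammo, UI image and sockets, back from its own values.
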(event `Disparar`)

(event `Recargar`)

(fn `UserConstructionScript`
  (bind (_damage _tamcargador _totalbalas _balasactuales _imagenui _socketdescanso _socketactivo) (break `/Game/EstructurasDeControl/Structs/InfoArmas` (`self.InfoDelArma`)))
  (`parent.UserConstructionScript`)
  (set `self.SePudeCojer?` true)
  (setmembers `/Game/EstructurasDeControl/Structs/InfoArmas` :`StructRef` (`self.InfoDelArma`) :`Damage` _damage :`TamCargador` _tamcargador :`TotalBalas` _totalbalas :`BalasActuales` _balasactuales :`ImagenUI` _imagenui :`SocketDescanso` _socketdescanso :`SocketActivo` _socketactivo)
  (set `self.TipoDeArma` "NewEnumerator0"))