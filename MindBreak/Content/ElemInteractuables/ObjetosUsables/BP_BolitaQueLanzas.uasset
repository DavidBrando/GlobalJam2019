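; BP_BolitaQueLanzas is a usable object: a small ball that gets thrown when used.
; RealizaTuUso enables physics on the mesh and applies an impulse along the given direction, then prints a debug string and destroys the actor after a short delay.
; The construction script calls the parent's, then sets TipoDeObjeto to mark the object's type.
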(event `self.RealizaTuUso`
  (params (Direction :type "Vector Structure"))
  (bind _mesh (`self.Mesh`))
  (`PrimitiveComponent.SetSimulatePhysics` _mesh true)
  (`PrimitiveComponent.AddImpulse` _mesh (* Direction 500.0) "None" false)
  (`KismetSystemLibrary.Delay` 5.0)
  (`KismetSystemLibrary.PrintString` "Shinee, Kakyoin!")
  (`self.K2_DestroyActor`))

(fn `UserConstructionScript`
  (`parent.UserConstructionScript`)
  (set `self.TipoDeObjeto` "NewEnumerator1"))