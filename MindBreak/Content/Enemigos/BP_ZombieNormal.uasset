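; BP_ZombieNormal is a standard zombie enemy that relies on its parent class for BeginPlay and Tick behavior.
; The construction script calls Inicializar to set its alive state, health and damage.
; It then picks a random BlendSelector from three values, and only the highest also sets a specific max walk speed on CharacterMovement, giving variation between zombies.
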(event `self.ReceiveBeginPlay`
  (`parent.ReceiveBeginPlay`))

(event `self.ReceiveTick`
  (params (DeltaSeconds :type "Float (single-precision)"))
  (`parent.ReceiveTick` DeltaSeconds))

(event `Inicializar`
  (set `self.Vivo` true)
  (bind _output_get (set `self.Vida` 500.0))
  (set `self.VidaMax` _output_get)
  (set `self.Damage` 20.0))

(fn `UserConstructionScript`
  (`parent.UserConstructionScript`)
  (`self.Inicializar`)
  (bind _output_get (set `self.blendSelector` (`KismetMathLibrary.RandomIntegerInRange` 0 2)))
  (if (== _output_get 2)
    (set `CharacterMovementComponent.MaxWalkSpeed` 600.0 (`self.CharacterMovement`))))